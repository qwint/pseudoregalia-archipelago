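; BP_APInteractableAura is an AP Randomizer mod actor that shows a Niagara aura at the position of the actor it follows.
; Each tick it moves itself to the location of its Follow actor.
; SetClassification maps a classification value to one of three aura systems, which SetAura assigns to the Aura component.
; Despawn only hides the actor rather than destroying it.
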(event EventTick
  (params (DeltaSeconds :type Float%20%28single-precision%29))
  (Transformation|SetActorLocation (Transformation|GetActorLocation (Variables|Default|Getfollow)) false false))

(fn ConstructionScript)

(fn Despawn
  (Rendering|SetActorHiddenInGame true))

(fn SetClassification
  (params (classification :type Integer))
  (switch int classification
    (:1
      (CallFunction|SetAura "/Game/VFX/Systems/NS_GoldAura.NS_GoldAura"))
    (:2
      (CallFunction|SetAura "/Game/VFX/Systems/NS_CameraRingAuraSave.NS_CameraRingAuraSave"))
    (:3
      (CallFunction|SetAura "/Game/VFX/Systems/NS_PinkAura.NS_PinkAura"))))

(fn SetAura
  (params (niagara :type Niagara%20System%20Object%20Reference))
  (Class|NiagaraComponent|SetAsset (Variables|Default|GetAura) niagara true))