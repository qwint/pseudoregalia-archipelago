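; Mod actor for the AP randomizer that bridges its C++ side to the game.
; BeginPlay adds client, console and logo widgets, removes a softlock-prone Library save point, and skips the opening cutscene.
; AP functions spawn collectibles, show popups, and write upgrades (expanding progressive ones), keys and health to MV_GameInstance, updating player or HUD.
; Empty Tick runs C++ actions on the game thread; the input-bound slide-jump toggle is a stub.
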(event EventBeginPlay
  (Utilities|FlowControl|Sequence
    (:then_0
      (bind _returnvalue (Actor|GetActorOfClass "/Game/ThirdPerson/Player/BP_PlayerGoatMain.BP_PlayerGoatMain_C"))
      (Variables|Default|SetPlayerRef _returnvalue))
    (:then_1
      (bind _returnvalue_2 (UserInterface|CreateWidget "/Game/Mods/AP_Randomizer/APClientWidget.APClientWidget_C"))
      (UserInterface|Viewport|AddtoViewport _returnvalue_2 1)
      (Variables|Default|SetWidgetRef _returnvalue_2))
    (:then_2
      ;[1 1 1] Delete 2nd save point in library to prevent accidental softlocks
      (bind _returnvalue_3 (Game|GetCurrentLevelName true))
      (if (Utilities|Enum|Equal(Enum) _returnvalue_3 "Zone_Library")
        (bind _outactors (Actor|GetAllActorsOfClass "/Game/Blueprints/LevelActors/BP_SavePoint.BP_SavePoint_C"))
        (for _array_element _outactors
          (if (Utilities|Enum|Equal(Enum) (Utilities|GetObjectName _array_element) "BP_SavePoint_C_2")
            (Actor|DestroyActor _array_element)))))
    (:then_3
      ;[1 1 1] show ap logo on main menu
      (bind _returnvalue_4 (Game|GetCurrentLevelName true))
      (if (Utilities|Enum|Equal(Enum) _returnvalue_4 "TitleScreen")
        (bind _returnvalue_5 (UserInterface|CreateWidget "/Game/Mods/AP_Randomizer/AP_Logo.AP_Logo_C"))
        (UserInterface|Viewport|AddtoViewport _returnvalue_5 -2)))
    (:then_4
      ;[1 1 1] create console
      (bind _returnvalue_6 (UserInterface|CreateWidget "/Game/Mods/AP_Randomizer/AP_DeluxeConsole.AP_DeluxeConsole_C"))
      (UserInterface|Viewport|AddtoViewport _returnvalue_6 1))
    (:then_5
      ;[1 1 1] set opening cutscene as having already been watched
      (bind _asmv_game_instance (Utilities|Casting|CastToMV_GameInstance (Game|GetGameInstance)))
      (Utilities|Map|Add (Variables|/Game/Blueprints/GameData/MV_GameInstance.MV_GameInstance_C|GeteventTracker _asmv_game_instance) "opening" 1))))

(event EventTick
  (params (DeltaSeconds :type Float%20%28single-precision%29))
  ;[1 1 1] empty eventtick used for running actions in the game thread from c++
)

(event Input|GamepadEvents|GamepadFaceButtonTop
  (params (Key :type Key%20Structure))
  (:Pressed
    (CallFunction|APToggleSlideJump)))

(event Input|KeyboardEvents|LeftCtrl
  (params (Key :type Key%20Structure))
  (:Pressed
    (CallFunction|APToggleSlideJump)))

(fn ConstructionScript)

(fn APSpawnCollectible
  (params (collectible_id :type Integer64) (collectible_position :type Vector) (collectible_classification :type Integer))
  (bind _returnvalue (Game|SpawnActorfromClass "/Game/Mods/AP_Randomizer/BP_APCollectible.BP_APCollectible_C" (Math|Transform|MakeTransform (Math|Vector|MakeVector (.x collectible_position) (.y collectible_position) (+ (.z collectible_position) 1.5e+02)) "0, 0, 0" "1.000000,1.000000,1.000000") "Undefined" 0 0))
  (Variables|/Game/Mods/AP_Randomizer/BP_APCollectible.BP_APCollectible_C|Setid _returnvalue collectible_id)
  (Default|SetClassification _returnvalue collectible_classification)
  (return true))

(fn APSetUpgrades
  (params (new_name :type Array%20of%20Names) (new_count :type Array%20of%20Integers) (disable_slidejump :type Boolean))
  (bind _asmv_game_instance (Utilities|Casting|CastToMV_GameInstance (Game|GetGameInstance)))
  (LocalVariables|Setnew_map (Variables|/Game/Blueprints/GameData/MV_GameInstance.MV_GameInstance_C|GetupgradeTracker _asmv_game_instance))
  (for (_array_element _array_index) new_name
    (LocalVariables|Setcurrent_name _array_element)
    (LocalVariables|Setindex _array_index)
    (LocalVariables|Setcurrent_count (Utilities|Array|Get(acopy) new_count (LocalVariables|Getindex)))
    (if (not (>= (.Value (Utilities|Map|Find (LocalVariables|Getnew_map) (LocalVariables|Getcurrent_name))) (LocalVariables|Getcurrent_count)))
      (Utilities|Map|Add (LocalVariables|Getnew_map) (LocalVariables|Getcurrent_name) (LocalVariables|Getcurrent_count))))
  (Utilities|FlowControl|Sequence
    (:then_0
      ;[1 1 1] check for progressive slide
      (switch int (.Value (Utilities|Map|Find (LocalVariables|Getnew_map) "progressiveSlide"))
        (:Default
          (Utilities|Map|Add (LocalVariables|Getnew_map) "slide" 1 :!label _label)
          (Utilities|Map|Add (LocalVariables|Getnew_map) "SlideJump" 1))
        (:1
          (Utilities|Map|Add (LocalVariables|Getnew_map) "slide" 1))
        (:2
          (goto _label))))
    (:then_1
      ;[1 1 1] check for progressive breaker
      (switch int (.Value (Utilities|Map|Find (LocalVariables|Getnew_map) "progressiveBreaker"))
        (:1
          (Utilities|Map|Add (LocalVariables|Getnew_map) "attack" 1))
        (:2
          (Utilities|Map|Add (LocalVariables|Getnew_map) "attack" 1)
          (Utilities|Map|Add (LocalVariables|Getnew_map) "chargeAttack" 1))
        (:3
          (Utilities|Map|Add (LocalVariables|Getnew_map) "attack" 1)
          (Utilities|Map|Add (LocalVariables|Getnew_map) "chargeAttack" 1)
          (Utilities|Map|Add (LocalVariables|Getnew_map) "projectile" 1))))
    (:then_2
      ;[1 1 1] configure slide ui if slide + SlideJump
      (if (and (> (.Value (Utilities|Map|Find (LocalVariables|Getnew_map) "slide")) 0) (> (.Value (Utilities|Map|Find (LocalVariables|Getnew_map) "SlideJump")) 0))
        (CallFunction|ConfigureSlideUI disable_slidejump)))
    (:then_3
      ;[1 1 1] check for disabled slidejump
      (if disable_slidejump
        (Utilities|Map|Add (LocalVariables|Getnew_map) "SlideJump" 0)))
    (:then_4
      (bind _output_get (Variables|/Game/Blueprints/GameData/MV_GameInstance.MV_GameInstance_C|SetupgradeTracker _asmv_game_instance (LocalVariables|Getnew_map)))
      (Default|UpdateUpgrades (Variables|Default|GetPlayerRef) _output_get))))

(fn APSetMajorKeys
  (params (keys :type Array%20of%20Booleans))
  (bind _asmv_game_instance (Utilities|Casting|CastToMV_GameInstance (Game|GetGameInstance)))
  (for (_array_element _array_index) keys
    (switch int _array_index
      (:0
        (Variables|/Game/Blueprints/GameData/MV_GameInstance.MV_GameInstance_C|Setkey1 _asmv_game_instance _array_element))
      (:1
        (Variables|/Game/Blueprints/GameData/MV_GameInstance.MV_GameInstance_C|Setkey2 _asmv_game_instance _array_element))
      (:2
        (Variables|/Game/Blueprints/GameData/MV_GameInstance.MV_GameInstance_C|Setkey3 _asmv_game_instance _array_element))
      (:3
        (Variables|/Game/Blueprints/GameData/MV_GameInstance.MV_GameInstance_C|Setkey4 _asmv_game_instance _array_element))
      (:4
        (Variables|/Game/Blueprints/GameData/MV_GameInstance.MV_GameInstance_C|Setkey5 _asmv_game_instance _array_element)))))

(fn APSetSmallKeys
  (params (key_count :type Integer))
  (bind _asmv_game_instance (Utilities|Casting|CastToMV_GameInstance (Game|GetGameInstance)))
  (Utilities|FlowControl|Sequence
    (:then_0
      ;[1 1 1] Count how many doors have been unlocked, and store the sum in spent_keys
      (for _array_element (Variables|/Game/Blueprints/GameData/MV_GameInstance.MV_GameInstance_C|GetallZoneDataStrs _asmv_game_instance)
        (bind _keys (Utilities|Map|Keys (.namesAndStates (Utilities|Struct|BreakST_ZoneData _array_element))))
        (for _array_element_2 _keys
          (if (Utilities|String|StartsWith _array_element_2 "BP_LockDoor")
            (LocalVariables|Setspent_keys (+ (LocalVariables|Getspent_keys) (.Value (Utilities|Map|Find (.namesAndStates (Utilities|Struct|BreakST_ZoneData _array_element)) _array_element_2))))))))
    (:then_1
      ;[1 1 1] Set NumberOfKeys to key_count - spent_keys.
      (bind _output_get (Variables|/Game/Blueprints/GameData/MV_GameInstance.MV_GameInstance_C|SetNumberOfKeys _asmv_game_instance (- key_count (LocalVariables|Getspent_keys))))
      (bind _foundwidgets (Widget|GetAllWidgetsOfClass "/Game/UI/UI_HUD.UI_HUD_C" true))
      (Default|UpdateKeyCountUI _foundwidgets _output_get))))

(fn APSetHealthPieces
  (params (healthpiece_count :type Integer))
  (bind _playerref (Variables|Default|GetPlayerRef))
  (bind _playerref_2 (Variables|Default|GetPlayerRef))
  (bind _bp_hphitable (Variables|/Game/ThirdPerson/Player/BP_PlayerGoatMain.BP_PlayerGoatMain_C|GetBP_HpHitable _playerref))
  (bind _bp_hphitable_2 (Variables|/Game/ThirdPerson/Player/BP_PlayerGoatMain.BP_PlayerGoatMain_C|GetBP_HpHitable _playerref_2))
  (bind _asmv_game_instance (Utilities|Casting|CastToMV_GameInstance (Game|GetGameInstance)))
  (if true
    (Utilities|FlowControl|Sequence
      (:then_0
        (LocalVariables|Setnew_maxhp (Math|Conversions|ToFloat(Integer) (+ (* (/ healthpiece_count 3) 10) 30)))
        (if (> (LocalVariables|Getnew_maxhp) (Variables|/Game/Blueprints/BP_HpHitable.BP_HpHitable_C|GetmaxHP (Variables|/Game/ThirdPerson/Player/BP_PlayerGoatMain.BP_PlayerGoatMain_C|GetBP_HpHitable (Variables|Default|GetPlayerRef))))
          ;[1 1 1] increase sybil's max hp
          (bind _output_get (Variables|/Game/Blueprints/GameData/MV_GameInstance.MV_GameInstance_C|SetmaxHP _asmv_game_instance (LocalVariables|Getnew_maxhp)))
          (bind _output_get_2 (Variables|/Game/Blueprints/BP_HpHitable.BP_HpHitable_C|SetmaxHP _bp_hphitable _output_get))
          (Variables|/Game/Blueprints/BP_HpHitable.BP_HpHitable_C|SetCurrentHP _bp_hphitable _output_get_2)
          (bind _foundwidgets (Widget|GetAllWidgetsOfClass "/Game/UI/UI_HUD.UI_HUD_C" true))
          (Default|UpdateCurrentHPValues _foundwidgets (Variables|/Game/Blueprints/BP_HpHitable.BP_HpHitable_C|GetCurrentHP _bp_hphitable_2) (Variables|/Game/ThirdPerson/Player/BP_PlayerGoatMain.BP_PlayerGoatMain_C|GetcurrentPower _playerref_2) (Variables|/Game/Blueprints/BP_HpHitable.BP_HpHitable_C|GetmaxHP _bp_hphitable_2) (Variables|/Game/ThirdPerson/Player/BP_PlayerGoatMain.BP_PlayerGoatMain_C|GetmaxPower _playerref_2) (Variables|/Game/ThirdPerson/Player/BP_PlayerGoatMain.BP_PlayerGoatMain_C|GetpowerLevel _playerref_2))))
      (:then_1
        (Variables|/Game/Blueprints/GameData/MV_GameInstance.MV_GameInstance_C|SethpPieces _asmv_game_instance healthpiece_count)))))

(fn APPrintMessage
  (params (new_text :type Text) (mute_sound :type Boolean))
  (bind _returnvalue (UserInterface|CreateWidget "/Game/UI/UI_MiniPopup.UI_MiniPopup_C"))
  (Default|SetInfo _returnvalue new_text)
  (Class|TextBlock|SetFont (Variables|/Game/UI/UI_MiniPopup.UI_MiniPopup_C|GetDescriptionText_1 _returnvalue) (Variables|Default|Getcyberbit_font))
  (Class|Widget|SetRenderTranslation (Variables|/Game/UI/UI_MiniPopup.UI_MiniPopup_C|GetDescriptionText_1 _returnvalue) "(X=-75.000000,Y=0.000000)")
  (Class|Widget|SetRenderTranslation _returnvalue "(X=250.000000,Y=-100.000000)")
  (Class|Widget|SetRenderTransformAngle _returnvalue 1.8e+02)
  (Widget|Transform|SetRenderScale _returnvalue "(X=0.750000,Y=0.750000)")
  (Widget|Panel|AddChild (Variables|/Game/Mods/AP_Randomizer/APClientWidget.APClientWidget_C|Getwidget_text_container (Variables|Default|GetWidgetRef)) _returnvalue)
  (if (not mute_sound)
    (Audio|PlaySound2D "/Game/Audio/Sounds/cue_keyGet.cue_keyGet" 0.8 1.0 0.0 0 0)))

(fn APToggleSlideJump
  (return))

(fn ConfigureSlideUI
  (params (slide :type Boolean))
  ;[1 1 1] don't add widget to a non gameplay level
  (bind _returnvalue (Game|GetCurrentLevelName true))
  (if (not (or (Utilities|Enum|Equal(Enum) _returnvalue "TitleScreen") (Utilities|Enum|Equal(Enum) _returnvalue "EndScreen")))
    (Utilities|FlowControl|Sequence
      (:then_0
        (Utilities|IsValid (Variables|Default|GetSlideIconRef)
          (:Is%20Not%20Valid
            (bind _returnvalue_2 (UserInterface|CreateWidget "/Game/Mods/AP_Randomizer/AP_SlideIcon.AP_SlideIcon_C"))
            (bind _output_get (Variables|Default|SetSlideIconRef _returnvalue_2))
            (UserInterface|Viewport|AddtoViewport _output_get -1))))
      (:then_1
        (Default|SetIcon (Variables|Default|GetSlideIconRef) slide)))))

(fn APPrintItemMessage
  (params (preamble :type Text) (item :type Text) (info :type Text) (mute_sound :type Boolean))
  (bind _returnvalue (UserInterface|CreateWidget "/Game/UI/UI_MiniPopup.UI_MiniPopup_C"))
  (Default|SetInfo _returnvalue preamble item info)
  (Class|Widget|SetRenderTranslation _returnvalue "(X=60.000000,Y=-50.000000)")
  (Class|Widget|SetRenderTransformAngle _returnvalue 1.8e+02)
  (Widget|Panel|AddChild (Variables|/Game/Mods/AP_Randomizer/APClientWidget.APClientWidget_C|Getwidget_text_container (Variables|Default|GetWidgetRef)) _returnvalue)
  (if (not mute_sound)
    (Audio|PlaySound2D "/Game/Audio/Sounds/cue_keyGet.cue_keyGet" 0.8 1.0 0.0 0 0)))