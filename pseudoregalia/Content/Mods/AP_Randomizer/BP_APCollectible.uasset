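; Archipelago randomizer collectible pickup that passes its Id to ReturnCheck, an empty stub here, when the player goat overlaps its sphere.
; SetClassification sets its look by item type: AP logo with a Niagara aura for generic items, aura alone for abilities and aspects, configured meshes for keys and health pieces.
; Tick billboards the sprite toward the camera.
; Despawn hides the actor and disables sphere collision, but nothing here calls it.
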(event OnComponentBeginOverlap(Sphere)
  (params (OverlappedComponent :type Primitive%20Component%20Object%20Reference) (OtherActor :type Actor%20Object%20Reference) (OtherComp :type Primitive%20Component%20Object%20Reference) (OtherBodyIndex :type Integer) (bFromSweep :type Boolean) (SweepResult :type Hit%20Result%20Structure%20%28by%20ref%29))
  (if (Utilities|Enum|Equal(Enum) (Utilities|GetClassDisplayName (Utilities|GetClass OtherActor)) "BP_PlayerGoatMain_C")
    (CallFunction|ReturnCheck (Variables|Default|Getid))))

(event EventTick
  (params (DeltaSeconds :type Float%20%28single-precision%29))
  (Transformation|SetWorldRotation (Variables|Default|GetSprite) (Math|Rotator|FindLookatRotation (Transformation|GetActorLocation) (Camera|GetCameraLocation (Variables|Default|GetCam%20Ref))) false false))

(event EventBeginPlay
  (Variables|Default|SetCam%20Ref (Game|GetPlayerCameraManager 0)))

(fn ConstructionScript)

(fn ReturnCheck
  (params (id :type Integer64))
  (return))

(fn Despawn
  (Rendering|SetActorHiddenInGame true)
  (Collision|SetCollisionEnabled (Variables|Default|GetSphere) "NoCollision"))

(fn SetClassification
  (params (classification :type Integer))
  (switch int classification
    (:Default
      ;[1 1 1] generic
      (CallFunction|ShowSprite)
      (CallFunction|SetAura "/Game/VFX/Systems/NS_Healing.NS_Healing"))
    (:1
      ;[1 1 1] generic progression
      (CallFunction|ShowSprite)
      (CallFunction|SetAura "/Game/VFX/Systems/NS_GoldAura.NS_GoldAura"))
    (:2
      ;[1 1 1] generic useful/trap
      (CallFunction|ShowSprite)
      (CallFunction|SetAura "/Game/VFX/Systems/NS_CameraRingAuraSave.NS_CameraRingAuraSave"))
    (:3
      ;[1 1 1] generic filler
      (CallFunction|ShowSprite)
      (CallFunction|SetAura "/Game/VFX/Systems/NS_PinkAura.NS_PinkAura"))
    (:4
      ;[1 1 1] ability
      (CallFunction|SetAura "/Game/VFX/Systems/NS_WhiteAura1.NS_WhiteAura1"))
    (:5
      ;[1 1 1] aspect
      (CallFunction|SetAura "/Game/VFX/Systems/NS_SmallUpgradeAura.NS_SmallUpgradeAura"))
    (:6
      ;[1 1 1] health piece
      (CallFunction|SetAura "/Game/VFX/Systems/NS_PinkAura.NS_PinkAura")
      (CallFunction|ConfigureHealthPieceMesh))
    (:7
      ;[1 1 1] major key
      (CallFunction|SetAura "/Game/VFX/Systems/NS_GoldAura.NS_GoldAura")
      (CallFunction|ConfigureMajorKeyMesh))
    (:8
      ;[1 1 1] small key
      (CallFunction|ConfigureSmallKeyMesh))))

(fn SetAura
  (params (NewParam :type Niagara%20System%20Object%20Reference))
  (Class|NiagaraComponent|SetAsset (Variables|Default|GetAura) NewParam true)
  (Rendering|SetVisibility (Variables|Default|GetAura) true true))

(fn ShowSprite
  (Rendering|SetVisibility (Variables|Default|GetAP%20Logo) true true))

(fn ConfigureMajorKeyMesh
  (Components|StaticMesh|SetStaticMesh (Variables|Default|GetMesh) "/Game/Meshes/Environment/Props/bigKey.bigKey")
  (Rendering|Material|SetMaterial (Variables|Default|GetMesh) 0 "/Game/MatTex/Materials/M_BigKey.M_BigKey")
  (Transformation|SetRelativeRotation (Variables|Default|GetMesh) "-40.000000,0.000000,0.000000" false false)
  (Rendering|SetVisibility (Variables|Default|GetMesh) true true))

(fn ConfigureSmallKeyMesh
  (Components|StaticMesh|SetStaticMesh (Variables|Default|GetMesh) "/Game/Meshes/Environment/Props/smallKey.smallKey")
  (Rendering|Material|SetMaterial (Variables|Default|GetMesh) 0 "/Game/MatTex/Materials/M_SmallKey.M_SmallKey")
  (Transformation|SetRelativeRotation (Variables|Default|GetMesh) "-40.000000,0.000000,0.000000" false false)
  (Rendering|SetVisibility (Variables|Default|GetMesh) true true))

(fn ConfigureHealthPieceMesh
  (Components|StaticMesh|SetStaticMesh (Variables|Default|GetMesh) "/Game/Meshes/Environment/Props/hpUpgradeMesh.hpUpgradeMesh")
  (Rendering|Material|SetMaterial (Variables|Default|GetMesh) 0 "/Game/MatTex/Materials/M_BigKey.M_BigKey")
  (Transformation|SetRelativeScale3D (Variables|Default|GetMesh) "1.250000,1.250000,1.250000")
  (Rendering|SetVisibility (Variables|Default|GetMesh) true true))